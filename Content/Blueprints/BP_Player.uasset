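; BP_Player is the player-controlled pawn, with look controls, planar movement and access to the game menu.
; Forward and right input move it by swept, frame-time-scaled world offsets along control-rotation yaw, ignoring pitch and roll.
; Number keys 1–4 select preset speeds.
; The GameMenu action disables input, fetches WBP_Menu from the HUD through a message call, displays it and shows the cursor.
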(event `InputAxis|Turn` :overrideparent false
  (params (AxisValue :type "Float (single-precision)"))
  (`self.AddControllerYawInput` AxisValue))

(event `Key|One`
  (params (Key :type "Key Structure"))
  ;[1 1 1] Change Speed
  (:`Pressed`
    (set `self.MultiplySpeed` 700.0)))

(event `Key|Two`
  (params (Key :type "Key Structure"))
  ;[1 1 1] Change Speed
  (:`Pressed`
    (set `self.MultiplySpeed` 1200.0)))

(event `InputAxis|LookUp` :overrideparent false
  (params (AxisValue :type "Float (single-precision)"))
  (`self.AddControllerPitchInput` AxisValue))

(event `Key|Four`
  (params (Key :type "Key Structure"))
  ;[1 1 1] Change Speed
  (:`Pressed`
    (set `self.MultiplySpeed` 2200.0)))

(event `Key|Three`
  (params (Key :type "Key Structure"))
  ;[1 1 1] Change Speed
  (:`Pressed`
    (set `self.MultiplySpeed` 1700.0)))

(event `InputAction|GameMenu`
  (params (Key :type "Key Structure"))
  (:`Pressed`
    (`self.DisableInput` (cast `PlayerController` (`self.GetController`) :!pure true))
    (`WidgetBlueprintLibrary.SetInputMode_GameAndUIEx` (cast `PlayerController` (`self.GetController`) :!pure true) null "DoNotLock" false)
    (bind _getwidget (message `/Game/Blueprints/Interface/BPI_HUD.GetWidgetsFromHUD` (`PlayerController.GetHUD` (cast `PlayerController` (`self.GetController`) :!pure true))))
    (bind _aswbp_menu (cast `/Game/Widgets/WBP_Menu` _getwidget))
    (`UserWidget.AddToViewport` _aswbp_menu 0)
    (set `PlayerController.bShowMouseCursor` true (cast `PlayerController` (`self.GetController`) :!pure true))))

(event `InputAxis|MoveForward` :overrideparent false
  (params (AxisValue :type "Float (single-precision)"))
  (`self.K2_AddActorWorldOffset` (* (`KismetMathLibrary.GetForwardVector` (`KismetMathLibrary.MakeRotator` 0.0 0.0 (.yaw (`self.GetControlRotation`)))) (* AxisValue (`self.MultiplySpeed`) (`GameplayStatics.GetWorldDeltaSeconds`))) true))

(event `InputAxis|MoveRight` :overrideparent false
  (params (AxisValue :type "Float (single-precision)"))
  (`self.K2_AddActorWorldOffset` (* (`KismetMathLibrary.GetRightVector` (`KismetMathLibrary.MakeRotator` 0.0 0.0 (.yaw (`self.GetControlRotation`)))) (* AxisValue (`self.MultiplySpeed`) (`GameplayStatics.GetWorldDeltaSeconds`))) true))

(fn `UserConstructionScript`)